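; BP_FPSHUB is a first-person HUD Blueprint that puts the player's on-screen UI and crosshair in place.
; On BeginPlay it creates the WBP_FPSHUD widget and adds it to the viewport.
; Each DrawHUD call draws the Crosshair texture with a white tint, sized by CrosshairSize and centered using the screen dimensions.
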(event `self.ReceiveBeginPlay`
  ;[1 1 1] 绘制UI
  (bind _returnvalue (`|CreateWidget` "/Game/BluePrints/WBP_FPSHUD.WBP_FPSHUD_C"))
  (`UserWidget.AddToViewport` _returnvalue 0))

(event `self.ReceiveDrawHUD`
  (params (SizeX :type Integer) (SizeY :type Integer))
  (bind _crosshairsize (`self.CrosshairSize`))
  (bind _returnvalue (`KismetMathLibrary.Conv_IntToDouble` _crosshairsize))
  (bind _returnvalue_2 (/ _crosshairsize 2))
  ;[1 1 1] 绘制准心
  (`self.DrawTexture` "/Game/Graphics/crosshair.crosshair" (`KismetMathLibrary.Conv_IntToDouble` (- (/ SizeX 2) _returnvalue_2)) (`KismetMathLibrary.Conv_IntToDouble` (- (/ SizeY 2) _returnvalue_2)) _returnvalue _returnvalue 0.0 0.0 1.0 1.0 (make `LinearColor` 1.0 1.0 1.0 1.0) "BLEND_Translucent" 1.0 true))

(fn `UserConstructionScript`)