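; BP_Projectile is a projectile that reacts on hit with a bullet impact effect and destroys itself after a short delay.
; The Hit event spawns the particle at the hit location, then checks whether the struck component simulates physics.
; Only then does it push the component with a velocity-scaled impulse and call ApplyDamage, which has no damaged actor connected.
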(event `self.ReceiveHit`
  (params (MyComp :type "PrimitiveComponent Object Reference") (Other :type "Actor Object Reference") (OtherComp :type "PrimitiveComponent Object Reference") (bSelfMoved :type Boolean) (HitLocation :type "Vector Structure") (HitNormal :type "Vector Structure") (NormalImpulse :type "Vector Structure") (Hit :type "HitResult Structure (by ref)"))
  (`GameplayStatics.SpawnEmitterAtLocation` "/Game/BlockBreaker/ParticleSystems/PS_BulletImpact.PS_BulletImpact" HitLocation)
  (if (`SceneComponent.IsSimulatingPhysics` OtherComp "None")
    (`PrimitiveComponent.AddImpulseAtLocation` OtherComp (* (`self.GetVelocity`) 15) (`self.K2_GetActorLocation`) "None")
    (`GameplayStatics.ApplyDamage` null (`self.Damage`)))
  (`KismetSystemLibrary.Delay` 0.1)
  (`self.K2_DestroyActor`))

(fn `UserConstructionScript`)