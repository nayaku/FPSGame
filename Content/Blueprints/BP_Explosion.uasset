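; Explosion actor that plays a particle and sound effect at its location on spawn, then destroys itself after a short delay.
; The first actor overlap fires Bomb once, applying full radial damage on the authority only, with tunable damage and radius.
; Damage skips the explosion itself and a designated IgnoredActor, and names the overlapping actor as damage causer.
; A debug "bomb" string prints on each detonation.
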(event `self.ReceiveBeginPlay`
  (bind (_returnvalue_location _returnvalue_rotation) (`KismetMathLibrary.BreakTransform` (`self.GetTransform`)))
  (`KismetArrayLibrary.Array_Add` (`self.ignoredActors`) self)
  (`KismetArrayLibrary.Array_Add` (`self.ignoredActors`) (`self.IgnoredActor`))
  (`GameplayStatics.SpawnEmitterAtLocation` "/Game/FPS_Game/Particles/P_Explosion.P_Explosion" _returnvalue_location _returnvalue_rotation)
  (`GameplayStatics.SpawnSoundAtLocation` "/Game/StarterContent/Audio/Explosion01.Explosion01" (`self.K2_GetActorLocation`) (struct) 1.0 1.0 0.0 null null)
  (`KismetSystemLibrary.Delay` 2.0)
  (`self.K2_DestroyActor`))

(event `self.ReceiveActorBeginOverlap`
  (params (OtherActor :type "Actor Object Reference"))
  (`/Engine/EditorBlueprintResources/StandardMacros.DoOnce` false
    (:`Completed`
      (`self.Bomb`))))

(event `Bomb`
  (`/Engine/EditorBlueprintResources/ActorMacros.Switch Has Authority`
    (:`Authority`
      (`GameplayStatics.ApplyRadialDamage` (`self.ExplosionDamage`) (`self.K2_GetActorLocation`) (`self.DamageRadius`) null (`self.ignoredActors`) (stale `self.ReceiveActorBeginOverlap` OtherActor) null true)
      (`KismetSystemLibrary.PrintString` "bomb"))))

(fn `UserConstructionScript`)