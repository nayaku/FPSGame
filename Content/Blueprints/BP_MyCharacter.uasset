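; First-person player character that handles movement, look, jumping, sprinting, shooting, grenade throws, a flashlight toggle and quitting.
; BeginPlay spawns a pistol attached to the arms mesh's GripPoint.
; Held fire is polled on Tick, shooting from the camera, gated by the gun's fire-rate delay and blocked while sprinting.
; Sprint, started only on the ground, changes walk speed and drives a CameraShake subgraph that sets the sprint state.
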(event `InputAxis|MoveForward`
  (params (AxisValue :type "Float (single-precision)"))
  ;[1 1 1] 移动
  (`self.AddMovementInput` (`self.GetActorForwardVector`) AxisValue))

(event `InputAction|Fire`
  (params (Key :type "Key Structure"))
  ;[1 1 1] 射击
  (:`Pressed`
    (set `self.FireButtonDown` true))
  (:`Released`
    (set `self.FireButtonDown` false)))

(event `InputAction|ExitGame`
  (params (Key :type "Key Structure"))
  ;[1 1 1] 退出游戏
  (:`Released`
    (`KismetSystemLibrary.QuitGame` null "Quit")))

(event `self.ReceiveTick`
  (params (DeltaSeconds :type "Float (single-precision)"))
  (bind _firstpersoncamera (`self.FirstPersonCamera`))
  (bind _returnvalue (`SceneComponent.K2_GetComponentLocation` _firstpersoncamera))
  ;[1 1 1] 射击
  (if (and (`self.FireButtonDown`) (`self.CanShoot`) (not (`self.IsSprint`)))
    (`/Game/BluePrints/BP_WeaponBase.Shoot` (`self.EquippedGun`) _returnvalue (+ _returnvalue (* (`SceneComponent.GetForwardVector` _firstpersoncamera) (`/Game/BluePrints/BP_WeaponBase.MaxBulletDistance` (`self.EquippedGun`)))) (`KismetMathLibrary.MakeTransform` _returnvalue (`SceneComponent.K2_GetComponentRotation` _firstpersoncamera)))
    (set `self.CanShoot` false)
    (`KismetSystemLibrary.Delay` (`/Game/BluePrints/BP_WeaponBase.FireRate` (`self.EquippedGun`)))
    (set `self.CanShoot` true)))

(event `InputAxis|MoveRight`
  (params (AxisValue :type "Float (single-precision)"))
  ;[1 1 1] 移动
  (`self.AddMovementInput` (`self.GetActorRightVector`) AxisValue))

(event `InputAxis|Turn`
  (params (AxisValue :type "Float (single-precision)"))
  ;[1 1 1] 转向
  (`self.AddControllerYawInput` AxisValue))

(event `InputAxis|Lookup`
  (params (AxisValue :type "Float (single-precision)"))
  ;[1 1 1] 转向
  (`self.AddControllerPitchInput` AxisValue))

(event `self.ReceiveBeginPlay`
  ;[1 1 1] 装备武器
  (bind _returnvalue (`|SpawnActorFromClass` "/Game/BluePrints/BP_Pistol.BP_Pistol_C" (`KismetMathLibrary.Conv_VectorToTransform` (0.0 0.0 0.0)) "Undefined" "OverrideRootScale" null null))
  (`self.SetOwner` _returnvalue self)
  (`self.K2_AttachToComponent` _returnvalue (`self.Mesh_FPP`) "GripPoint" "SnapToTarget" "SnapToTarget" "SnapToTarget" true)
  (set `self.EquippedGun` _returnvalue))

(event `InputAction|Jump`
  (params (Key :type "Key Structure"))
  ;[1 1 1] 跳跃
  (:`Pressed`
    (`self.Jump`)
    (set `self.JumpButtonDown` (`self.CanJump`))
    (bind `_as角色移动组件` (cast `CharacterMovementComponent` (`self.GetMovementComponent`) :!label _label))
    (set `CharacterMovementComponent.JumpZVelocity` 400.0 `_as角色移动组件`))
  (:`Released`
    (`self.StopJumping`)
    (set `self.JumpButtonDown` false)
    (goto _label)))

(event `InputAction|OpenFlashlight`
  (params (Key :type "Key Structure"))
  ;[1 1 1] 开关手电筒
  (:`Pressed`
    (set `self.IsFlashlightOpen` (not (`self.IsFlashlightOpen`)))
    (`SceneComponent.SetVisibility` (`/Game/BluePrints/BP_WeaponBase.Flashlight` (`self.EquippedGun`)) (`self.IsFlashlightOpen`) false)))

(event `InputAction|Sprint`
  (params (Key :type "Key Structure"))
  (bind _charactermovement (`self.CharacterMovement`))
  ;[1 1 1] 冲刺
  (:`Pressed`
    (if (not (`NavMovementComponent.IsFalling` (`self.CharacterMovement`)))
      (set `CharacterMovementComponent.MaxWalkSpeed` (`self.SpeedSprint`) _charactermovement)
      (`self.CameraShake` :!label _label_2
        (:`Sprinting`
          (set `self.IsSprint` true))
        (:`Walking`
          (set `self.IsSprint` false)))))
  (:`Released`
    (if (`self.IsSprint`)
      (set `CharacterMovementComponent.MaxWalkSpeed` (`self.SpeedWalking`) _charactermovement)
      (goto _label_2 :!via `Stop`))))

(event `InputAction|ThrowGrenade`
  (params (Key :type "Key Structure"))
  ;[1 1 1] 丢手雷
  (:`Pressed`
    (`|SpawnActorFromClass` "/Game/BluePrints/BP_GrenadeBase.BP_GrenadeBase_C" (`SceneComponent.K2_GetComponentToWorld` (`self.FirstPersonCamera`)) "AlwaysSpawn" "OverrideRootScale" null null)))

(fn `UserConstructionScript`)